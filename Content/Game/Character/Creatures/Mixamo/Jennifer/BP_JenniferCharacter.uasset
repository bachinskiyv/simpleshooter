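; Character Blueprint for Jennifer that handles her footstep and landing sounds and her animated weapon switching.
; On BeginPlay it binds to footstep, landing and weapon-swap dispatchers on ABP_Jennifer, playing movement sounds at the bottom of the capsule.
; Equip begin plays the switch montage and an attached sound, while the actual EquipSync waits for the animation Blueprint's swap dispatcher.
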(event `self.ReceiveBeginPlay`
  (`|ExecutionSequence`
    (:`then_0`
      (bind _asabp_jennifer (cast `/Game/Game/Character/Creatures/Mixamo/Jennifer/ABP_Jennifer` (`SkeletalMeshComponent.GetAnimInstance` (`self.Mesh`))))
      (add `/Game/Game/Character/Creatures/Mixamo/Jennifer/ABP_Jennifer.FootstepsDispatcher` _asabp_jennifer (delegate `Footsteps`))
      (add `/Game/Game/Character/Creatures/Mixamo/Jennifer/ABP_Jennifer.LandingDispatcher` _asabp_jennifer (delegate `Landing`))
      (add `/Game/Game/Character/Creatures/Mixamo/Jennifer/ABP_Jennifer.SwapWeaponDispatcher` _asabp_jennifer (delegate `SwapWeapon`)))))

(event `SwapWeapon`
  (`WeaponsInventoryComponent.EquipSync` (`self.WeaponsInventoryComponent`) (stale `self.WeaponsInventoryComponent.OnEquipBegin` WeaponClass)))

(event `Footsteps`
  (`GameplayStatics.PlaySoundAtLocation` "/Game/Game/Character/Creatures/Mixamo/Jennifer/Audio/JenniferFootsteps.JenniferFootsteps" (- (`self.K2_GetActorLocation`) (`KismetMathLibrary.MakeVector` 0.0 0.0 (`CapsuleComponent.GetScaledCapsuleHalfHeight` (`self.CapsuleComponent`)))) (struct) 1.0 1.0 0.0 "/Game/Game/Character/Audio/ATT_Footsteps.ATT_Footsteps" null self))

(event `Landing`
  (`GameplayStatics.PlaySoundAtLocation` "/Game/Game/Character/Creatures/Mixamo/Jennifer/Audio/Jennifer_Landing.Jennifer_Landing" (- (`self.K2_GetActorLocation`) (`KismetMathLibrary.MakeVector` 0.0 0.0 (`CapsuleComponent.GetScaledCapsuleHalfHeight` (`self.CapsuleComponent`)))) (struct) 1.0 1.0 0.0 "/Game/Game/Character/Audio/ATT_Footsteps.ATT_Footsteps" null self))

(event `self.WeaponsInventoryComponent.OnEquipBegin`
  (params (WeaponClass :type "Weapon Class Reference"))
  (`self.PlayAnimMontage` "/Game/Game/Character/Creatures/Mixamo/Jennifer/Anims/JenniferSwitchWeapon.JenniferSwitchWeapon" 1.5)
  (`GameplayStatics.SpawnSoundAttached` "/Game/Game/Character/Audio/S_Swap_Weapon.S_Swap_Weapon" (`self.Mesh`) "None" (0.0 0.0 0.0) (struct) "KeepRelativeOffset" false 1.0 1.0 0.0 "/Game/Game/Character/Audio/ATT_Footsteps.ATT_Footsteps" null))

(fn `UserConstructionScript`
  (`parent.UserConstructionScript`))