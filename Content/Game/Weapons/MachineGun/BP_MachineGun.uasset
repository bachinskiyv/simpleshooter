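; Machine gun weapon Blueprint that adds audio and visual feedback for firing and bullet impacts.
; BeginPlay binds the fire and trace-hit delegates and pre-attaches an inactive muzzle flash emitter to the mesh socket.
; Each shot plays a sound and toggles that reused emitter for the time between shots.
; Trace hits spawn impact sound and particles, plus a short-lived attached decal unless a ShooterCharacter is hit.
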(event `OnFireDelegate_Event`
  (`GameplayStatics.SpawnSoundAtLocation` "/Game/Game/Weapons/MachineGun/Audio/S_Machinegun_Shot.S_Machinegun_Shot" (`self.K2_GetActorLocation`) (struct) 1.0 1.0 0.0 "/Game/Game/Character/Audio/ATT_Weapon.ATT_Weapon" null)
  (`ActorComponent.Activate` (stale `self.ReceiveBeginPlay` _returnvalue) true)
  (`KismetSystemLibrary.Delay` (`self.TimeBetweenShoots`))
  (`ActorComponent.Deactivate` (stale `self.ReceiveBeginPlay` _returnvalue)))

(event `OnTraceHit`
  (params (HitResult :type "HitResult Structure") (bDamageWasApplied :type Boolean))
  (`self.SpawnEffectsOnTraceHit` HitResult))

(event `self.ReceiveBeginPlay`
  (add `InstantHitWeapon.OnTraceHitDelegate` (delegate `OnTraceHit`))
  (bind _returnvalue (`GameplayStatics.SpawnEmitterAttached` "/Game/AssetPacks/ShooterGame/Effects/ParticleSystems/Weapons/AssaultRifle/Muzzle/P_AssaultRifle_MF.P_AssaultRifle_MF" (`self.Mesh`) "MuzzleFlashSocket" (0.0 0.0 0.0) (struct) (1.0 1.0 1.0) "KeepRelativeOffset" false "None" false))
  (add `self.OnFireDelegate` (delegate `OnFireDelegate_Event`)))

(fn `SpawnEffectsOnTraceHit`
  (params (Hit :type "HitResult Structure") (`Damage Was Applied` :type Boolean))
  (bind (_bblockinghit _binitialoverlap _time _distance _location _impactpoint _normal _impactnormal _physmat _hitactor _hitcomponent) (`GameplayStatics.BreakHitResult` Hit))
  (`GameplayStatics.PlaySoundAtLocation` "/Game/SFX/A_Impact_Cue.A_Impact_Cue" _location (struct) 0.5 1.0 0.0 "/Game/Game/Character/Audio/ATT_Weapon.ATT_Weapon" null null)
  (`GameplayStatics.SpawnEmitterAtLocation` "/Game/AssetPacks/ShooterGame/Effects/ParticleSystems/Weapons/AssaultRifle/Impacts/P_AssaultRifle_IH.P_AssaultRifle_IH" _location (`KismetMathLibrary.Conv_VectorToRotator` (* _normal -1.0)))
  (cast `ShooterCharacter` _hitactor
    (:`CastFailed`
      (`GameplayStatics.SpawnDecalAttached` "/Game/Game/Materials/M_RifleImpact.M_RifleImpact" (`KismetMathLibrary.Conv_DoubleToVector` 15.0) _hitcomponent "None" _location (`KismetMathLibrary.Conv_VectorToRotator` _location) "KeepWorldPosition" 8.0))))

(fn `UserConstructionScript`)