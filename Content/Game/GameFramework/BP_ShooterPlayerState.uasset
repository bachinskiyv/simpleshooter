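; Shooter player state Blueprint that composes kill message text from the killer and victim names.
; DetermineKillText casts the weapon class through machine gun, rocket launcher and rail rifle to pick a phrase, with a generic killed-by fallback.
; For the rocket launcher, the damage type class separates blast kills ("almost dodged") from other rocket kills ("rode").
; The event graph and construction script hold no active logic.
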(fn `DetermineKillText`
  (params (KillerName :type String) (VictimName :type String) (WeaponClass :type "Weapon Class Reference") (DamageTypeClass :type "DamageType Class Reference"))
  (returns (OutString :type String))
  (castclass `/Game/Game/Weapons/MachineGun/BP_MachineGun` WeaponClass
    (:`then`
      (return (`KismetStringLibrary.Concat_StrStr` VictimName " was machinegunned by " KillerName)))
    (:`CastFailed`
      (castclass `/Game/Game/Weapons/RocketLauncher/Blueprints/BP_RocketLauncher` WeaponClass
        (:`then`
          (castclass `/Game/Game/Weapons/RocketLauncher/Blueprints/DmgType_RocketBlast` DamageTypeClass
            (:`then`
              (return (`KismetStringLibrary.Concat_StrStr` VictimName " almost dodged " KillerName "'s rocket")))
            (:`CastFailed`
              (return (`KismetStringLibrary.Concat_StrStr` VictimName " rode " KillerName "'s rocket")))))
        (:`CastFailed`
          (castclass `/Game/Game/Weapons/Rail/Blueprints/BP_RailRifle` WeaponClass
            (:`then`
              (return (`KismetStringLibrary.Concat_StrStr` VictimName " was railed by " KillerName)))
            (:`CastFailed`
              (return (`KismetStringLibrary.Concat_StrStr` VictimName " was killed by " KillerName)))))))))

(fn `UserConstructionScript`)