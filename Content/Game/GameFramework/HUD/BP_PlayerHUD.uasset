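; BP_PlayerHUD is the player HUD that creates and owns the on-screen widgets for the shooter.
; On BeginPlay it adds the main HUD, a messages roulette and a scores widget to the viewport, taking the scores class from SimpleShooterGameModeBase and starting it collapsed.
; It exposes functions to toggle the scores widget and forward messages to the roulette.
; A debug print of widget names is left unwired.
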(event `self.ReceiveBeginPlay`
  (`self.Spawn Widgets`))

(event `CustomEvent_0`
  (`KismetSystemLibrary.PrintString` (`KismetStringLibrary.Concat_StrStr` "[VARZ] MESS: " (`KismetSystemLibrary.GetDisplayName` (`self.Messages_Widget`)) " SCOR: " (`KismetSystemLibrary.GetDisplayName` (`self.ScoresWidget`)) " HUD " (`KismetSystemLibrary.GetDisplayName` (`self.HUD_Widget`))) true true (struct :`R` 1.0 :`G` 0.196413 :`A` 1.0)))

(fn `DrawMessage`
  (params (Message :type String))
  (bind _messages_widget (`self.Messages_Widget`))
  (`/Engine/EditorBlueprintResources/StandardMacros.IsValid` _messages_widget
    (:`Is Valid`
      (`/Game/Game/UI/Messages/WBP_MessagesRoulette.DrawMessage` _messages_widget Message))))

(fn `Spawn Widgets`
  (`|ExecutionSequence`
    (:`then_0`
      (bind _returnvalue (`|GenericCreateObject` "/Game/Game/UI/WBP_HUD.WBP_HUD_C" (`self.PlayerOwner`)))
      (`UserWidget.AddToViewport` _returnvalue 0)
      (set `self.HUD_Widget` _returnvalue))
    (:`then_1`
      (bind _returnvalue_2 (`|GenericCreateObject` "/Game/Game/UI/Messages/WBP_MessagesRoulette.WBP_MessagesRoulette_C" (`self.PlayerOwner`)))
      (`UserWidget.AddToViewport` _returnvalue_2 0)
      (set `self.Messages_Widget` _returnvalue_2))
    (:`then_2`
      (bind _assimple_shooter_game_mode_base (cast `SimpleShooterGameModeBase` (`GameplayStatics.GetGameMode`)))
      (bind _returnvalue_3 (`|GenericCreateObject` (`SimpleShooterGameModeBase.ScoresWidgetClass` _assimple_shooter_game_mode_base) self))
      ;[0.6835 1 0.2474] TODO: UserWidget subclass cannot be constructed
      (bind _asuser_widget (cast `UserWidget` _returnvalue_3))
      (bind _output_get (set `self.ScoresWidget` _asuser_widget))
      (`UserWidget.AddToViewport` _output_get 0)
      (`Widget.SetVisibility` _output_get "Collapsed"))))

(fn `ToggleScoresWidget`
  (params (IsVisible :type Boolean))
  (bind _scoreswidget (`self.ScoresWidget`))
  (if (`KismetSystemLibrary.IsValid` (`self.ScoresWidget`))
    (if IsVisible
      (`Widget.SetVisibility` _scoreswidget "Visible")
      (else
        (`Widget.SetVisibility` _scoreswidget "Collapsed")))))

(fn `UserConstructionScript`)