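; Main menu HUD that displays the main menu widget while it is active.
; On BeginPlay it constructs the MainMenuWidget for the owning player, adds it to the viewport, focuses it with UI-only input and shows the mouse cursor.
; On EndPlay it removes the stored widget, restores game-only input and hides the cursor on player controller 0.
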(event `self.ReceiveBeginPlay`
  (`self.LoadMainMenu`))

(event `self.ReceiveEndPlay`
  (params (EndPlayReason :type "EEndPlayReason Enum" :default "Destroyed"))
  (bind _returnvalue (`GameplayStatics.GetPlayerController` 0))
  (`|ExecutionSequence`
    (:`then_0`
      (`Widget.RemoveFromParent` (`self.MainMenuWidgetObject`)))
    (:`then_1`
      (`WidgetBlueprintLibrary.SetInputMode_GameOnly` _returnvalue))
    (:`then_2`
      (set `PlayerController.bShowMouseCursor` false _returnvalue))))

(fn `LoadMainMenu`
  (bind _returnvalue (`self.GetOwningPlayerController`))
  (bind _returnvalue_2 (`|GenericCreateObject` (`self.MainMenuWidget`) _returnvalue))
  (`UserWidget.AddToViewport` _returnvalue_2 0)
  (`WidgetBlueprintLibrary.SetInputMode_UIOnlyEx` _returnvalue _returnvalue_2)
  (set `PlayerController.bShowMouseCursor` true _returnvalue)
  (set `self.MainMenuWidgetObject` _returnvalue_2))

(fn `UserConstructionScript`)