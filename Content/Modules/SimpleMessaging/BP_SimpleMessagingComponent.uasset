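; BP_SimpleMessagingComponent is an actor component that connects its owner to a simple messaging exchange on the Game Mode.
; It subscribes through BPI_MessagesExchange, caches that reference, and publishes outgoing messages through it.
; Incoming messages are forwarded to the owner's BPI_MessageDrawer interface for display.
; ReceiveBroadcast branches on system and chat types but is unfinished: ReceiveSpecial is empty and the chat branch only checks the sender reference.
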(event `/Game/Modules/SimpleMessaging/Interfaces/BPI_MessagesListener.SubscribeOnMessages`
  (bind _asbpi_messages_exchange (cast `/Game/Modules/SimpleMessaging/Interfaces/BPI_MessagesExchange` (`GameplayStatics.GetGameMode`)))
  (bind _output_get (set `self.Exchange` _asbpi_messages_exchange))
  (`/Game/Modules/SimpleMessaging/Interfaces/BPI_MessagesExchange.Subscribe` _output_get self))

(event `/Game/Modules/SimpleMessaging/Interfaces/BPI_MessagesSender.SendMessage`
  (params (Message :type String) (SenderState :type "ShooterPlayerState Soft Object Reference") (Type :type "/Game/Modules/SimpleMessaging/EMessageType Enum" :default "NewEnumerator0"))
  (bind _exchange (`self.Exchange`))
  (`/Engine/EditorBlueprintResources/StandardMacros.IsValid` (`KismetSystemLibrary.Conv_InterfaceToObject` _exchange)
    (:`Is Valid`
      (`/Game/Game/GameFramework/GameModes/BP_FreeForAllGameMode.PublishMessage` _exchange Message SenderState Type))))

(event `/Game/Modules/SimpleMessaging/Interfaces/BPI_MessagesListener.ReceiveMessage`
  (params (Message :type String) (ReceiverState :type "ShooterPlayerState Soft Object Reference") (Type :type "/Game/Modules/SimpleMessaging/EMessageType Enum" :default "NewEnumerator0"))
  (bind _asbpi_message_drawer (cast `/Game/Modules/SimpleMessaging/Interfaces/BPI_MessageDrawer` (`self.GetOwner` self)))
  (`/Game/Modules/SimpleMessaging/Interfaces/BPI_MessageDrawer.DrawMessage` _asbpi_message_drawer Message ReceiverState Type))

(fn `ReceiveBroadcast`
  (params (Message :type String) (SenderState :type "ShooterPlayerState Soft Object Reference") (Type :type "/Game/Modules/SimpleMessaging/EMessageType Enum" :default "NewEnumerator0"))
  (switch `/Game/Modules/SimpleMessaging/EMessageType` Type
    (:`NewEnumerator0`
      (`self.ReceiveSpecial` Message SenderState))
    (:`NewEnumerator1`
      (if (`KismetSystemLibrary.IsValidSoftObjectReference` SenderState)
        _))))

(fn `ReceiveSpecial`
  (params (Message :type String) (SenderState :type "ShooterPlayerState Soft Object Reference") (Type :type "/Game/Modules/SimpleMessaging/EMessageType Enum" :default "NewEnumerator0")))